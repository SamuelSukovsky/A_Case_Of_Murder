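; BP_Item is an item actor that animates itself to a target component, either to be placed or simply attached.
; The construction script applies a configurable mesh and transform.
; MoveItem runs a timeline that lerps from the current transform to the target's, adding PlacedRotation when placing.
; On finish it attaches to the target, keeping world rotation if placed and snapping rotation otherwise.
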(event Custom|Move%20Item
  (params (Target :type Scene%20Component%20Object%20Reference%20%28by%20ref%29) (Place :type Boolean))
  (bind _returnvalue (Transformation|GetWorldTransform Target))
  (bind (_location _rotation) (Math|Transform|BreakTransform _returnvalue))
  (bind _alpha (Timeline|Move%20To%20Location PlayFromStart)
    (:Update
      (Transformation|SetActorTransform (Math|Transform|Lerp(Transform) (Transformation|GetActorTransform) (select Place (Math|Transform|MakeTransform _location (Math|Rotator|CombineRotators (Variables|Default|GetPlaced%20Rotation) _rotation) "1.000000,1.000000,1.000000") (Math|Transform|MakeTransform _location _rotation "1.000000,1.000000,1.000000")) _alpha)))
    (:Finished
      (Transformation|AttachComponentToComponent Target "None" "SnapToTarget" (select Place "KeepWorld" "SnapToTarget") "KeepWorld" false))))

(fn ConstructionScript
  (bind _mesh (Variables|Default|GetMesh))
  (Components|StaticMesh|SetStaticMesh _mesh (Variables|Default|GetItem%20Mesh))
  (Transformation|SetRelativeTransform _mesh (Variables|Default|GetMesh%20Transform) false false))