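; BP_EvidenceBoard is the evidence board puzzle in A Case of Murder, checking whether the player has placed the correct weapon and motive.
; Both slots' item-changed events trigger a comparison against the expected items once both are filled.
; Wrong pairs play incorrect-answer dialogue through the DialogueManager, via a gate that the first correct answer closes.
; That one-time success plays correct dialogue, then after a delay starts the first level sequence found.
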(event Custom|Check%20Items
  (bind _dialogue_manager (Variables|Default|GetDialogue%20Manager))
  (bind _weapon_slot (Variables|Items|GetWeapon%20Slot))
  (bind _motive_slot (Variables|Items|GetMotive%20Slot))
  (bind _item (Variables|/Game/ACaseOfMurder/Blueprints/BP_ItemPlacement.BP_ItemPlacement_C|GetItem _weapon_slot))
  (bind _item_2 (Variables|/Game/ACaseOfMurder/Blueprints/BP_ItemPlacement.BP_ItemPlacement_C|GetItem _motive_slot))
  (if (and (Utilities|IsValid _item) (Utilities|IsValid _item_2))
    (if (and (== _item (Variables|Items|GetWeapon)) (== _item_2 (Variables|Items|GetMotive)))
      (Utilities|FlowControl|DoOnce false
        (:Completed
          (Utilities|FlowControl|Sequence
            (:then_0
              (goto _label Close))
            (:then_1
              (Default|StartDialogue _dialogue_manager "/Game/ACaseOfMurder/Data/DA_Dialogue_BoardCorrect.DA_Dialogue_BoardCorrect")
              (Utilities|FlowControl|Delay 1e+01)
              (bind _returnvalue (Actor|GetActorOfClass "/Script/LevelSequence.LevelSequenceActor"))
              (Sequencer|Player|Play (Variables|/Script/LevelSequence.LevelSequenceActor|GetSequencePlayer _returnvalue) :!class /Script/MovieScene.MovieSceneSequencePlayer)))))
      (else
        (Utilities|FlowControl|Gate false :!label _label
          (:Exit
            (Default|StartDialogue _dialogue_manager "/Game/ACaseOfMurder/Data/DA_Dialogue_BoardIncorrect.DA_Dialogue_BoardIncorrect")))))))

(event EventBeginPlay
  (EventDispatchers|BindEventtoItemChanged (Variables|Items|GetWeapon%20Slot) (delegate Custom|Check%20Items))
  (bind _returnvalue (Actor|GetActorOfClass "/Game/ACaseOfMurder/Blueprints/BP_DialogueManager.BP_DialogueManager_C"))
  (Variables|Default|SetDialogue%20Manager _returnvalue))

(fn ConstructionScript)