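; BP_ItemPlacement is an interactable marker for an item placement spot, shown as a pulsing circle with a prompt widget.
; A looping timeline scales the circle, which BeginPlay turns invisible after the construction script colors it by ItemType.
; Sphere overlap with the player character toggles the widget.
; The FocusInteraction interface event reveals the circle with a custom depth stencil highlight and passes focus to WBP_NearestInteraction.
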(event OnComponentBeginOverlap(Sphere)
  (params (OverlappedComponent :type Primitive%20Component%20Object%20Reference) (OtherActor :type Actor%20Object%20Reference) (OtherComp :type Primitive%20Component%20Object%20Reference) (OtherBodyIndex :type Integer) (bFromSweep :type Boolean) (SweepResult :type Hit%20Result%20Structure%20%28by%20ref%29))
  ;[0.6445 0.8228 1 0.502] Local Overlap Event
  (if (== (Game|GetPlayerCharacter 0) OtherActor)
    (Utilities|Casting|CastToBP_InteractionCharacter OtherActor)
    (Development|SetHiddeninGame (Variables|Default|GetWidget) false false)))

(event OnComponentEndOverlap(Sphere)
  (params (OverlappedComponent :type Primitive%20Component%20Object%20Reference) (OtherActor :type Actor%20Object%20Reference) (OtherComp :type Primitive%20Component%20Object%20Reference) (OtherBodyIndex :type Integer))
  (bind _sm_itemplacementcircle (Variables|Default|GetSM_ItemPlacementCircle))
  (bind _widget (Variables|Default|GetWidget))
  ;[0.6445 0.8228 1 0.502] Local Overlap Event
  (if (== OtherActor (Game|GetPlayerCharacter 0))
    (Utilities|Casting|CastToBP_InteractionCharacter OtherActor)
    (Rendering|SetRenderCustomDepth _sm_itemplacementcircle false)
    (Rendering|SetCustomDepthStencilValue _sm_itemplacementcircle 0)
    (if (Rendering|IsVisible _widget)
      (Development|SetHiddeninGame _widget true false))))

(event EventBeginPlay
  ;[1 1 1 0.5] Begin Play
  (bind _aswbp_nearest_interaction (Utilities|Casting|CastToWBP_NearestInteraction (UserInterface|GetWidget (Variables|Default|GetWidget))))
  (Variables|Default|SetAs%20WBP%20Nearest%20Interaction _aswbp_nearest_interaction)
  (Rendering|Material|SetMaterial (Variables|Default|GetSM_ItemPlacementCircle) 0 (Variables|Default|GetMaterial%20Invisible))
  ;[0.3564 0.227 0.02315] Animation
  (bind _circle_scale (Timeline|Animation%20Timeline Play)
    (:Update
      (Transformation|SetRelativeScale3D (Variables|Default|GetSM_ItemPlacementCircle) (Math|Conversions|ToVector(Float) _circle_scale)))
    (:Finished
      (Components|Timeline|PlayfromStart (Variables|Default|GetAnimation%20Timeline)))))

(event EventFocusInteraction
  (params (Focused :type Boolean))
  (bind _sm_itemplacementcircle (Variables|Default|GetSM_ItemPlacementCircle))
  (bind _widget (Variables|Default|GetWidget))
  (bind _widget_2 (Variables|Default|GetWidget))
  ;[1 1 1 0.5] Focus Interaction (interface)
  (if Focused
    ;[0.6445 0.8228 1 0.502] Local Visual
    (Rendering|Material|SetMaterial _sm_itemplacementcircle 0 (Variables|Default|GetMaterial%20Visible))
    (Rendering|SetRenderCustomDepth _sm_itemplacementcircle true)
    (Rendering|SetCustomDepthStencilValue _sm_itemplacementcircle 2)
    (if (Rendering|IsVisible _widget_2)
      _
      (else
        (Development|SetHiddeninGame _widget_2 false false)))
    (Default|OnFocused (Variables|Default|GetAs%20WBP%20Nearest%20Interaction) true)
    (else
      (Rendering|Material|SetMaterial _sm_itemplacementcircle 0 (Variables|Default|GetMaterial%20Invisible))
      (Rendering|SetRenderCustomDepth _sm_itemplacementcircle false)
      (Rendering|SetCustomDepthStencilValue _sm_itemplacementcircle 0)
      (if (Rendering|IsVisible _widget)
        _
        (else
          (Development|SetHiddeninGame _widget true false)))
      (Default|OnFocused (Variables|Default|GetAs%20WBP%20Nearest%20Interaction) false))))

(fn ConstructionScript
  (bind _sm_itemplacementcircle (Variables|Default|GetSM_ItemPlacementCircle))
  (switch Utilities|FlowControl|Switch|SwitchonE_ItemType (Variables|Default|GetItem%20Type)
    (:NewEnumerator0
      (Rendering|Material|SetMaterial _sm_itemplacementcircle 0 "/AnimationSharing/AnimSharingRed.AnimSharingRed"))
    (:NewEnumerator1
      (Rendering|Material|SetMaterial _sm_itemplacementcircle 0 "/AnimationSharing/AnimSharingGreen.AnimSharingGreen"))
    (:NewEnumerator2
      (Rendering|Material|SetMaterial _sm_itemplacementcircle 0 "/AnimationSharing/AnimSharingBlue.AnimSharingBlue"))))