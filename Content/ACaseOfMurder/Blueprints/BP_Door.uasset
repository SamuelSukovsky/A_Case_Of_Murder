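; Interactable exit door that ends the game with the correct-ending dialogue when opened.
; A multicast switch on locked state plus held key plays a locked sound, unlocks and detaches the key, or opens.
; Opening clears input mappings, blacks out post-process, hides UI, fades ambient audio, starts dialogue and quits after a delay.
; A sphere overlap shows the interaction widget, while focus highlights the meshes through custom depth stencil.
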(event OnComponentBeginOverlap(Sphere)
  (params (OverlappedComponent :type Primitive%20Component%20Object%20Reference) (OtherActor :type Actor%20Object%20Reference) (OtherComp :type Primitive%20Component%20Object%20Reference) (OtherBodyIndex :type Integer) (bFromSweep :type Boolean) (SweepResult :type Hit%20Result%20Structure%20%28by%20ref%29))
  ;[0.6445 0.8228 1 0.502] Local Overlap Event
  (if (== (Game|GetPlayerCharacter 0) OtherActor)
    (Utilities|Casting|CastToBP_InteractionCharacter OtherActor)
    (Development|SetHiddeninGame (Variables|Default|GetWidget) false false)))

(event OnComponentEndOverlap(Sphere)
  (params (OverlappedComponent :type Primitive%20Component%20Object%20Reference) (OtherActor :type Actor%20Object%20Reference) (OtherComp :type Primitive%20Component%20Object%20Reference) (OtherBodyIndex :type Integer))
  (bind _staticmesh (Variables|Default|GetStaticMesh))
  (bind _widget (Variables|Default|GetWidget))
  ;[0.6445 0.8228 1 0.502] Local Overlap Event
  (if (== OtherActor (Game|GetPlayerCharacter 0))
    (Utilities|Casting|CastToBP_InteractionCharacter OtherActor)
    (Rendering|SetRenderCustomDepth _staticmesh false)
    (Rendering|SetCustomDepthStencilValue _staticmesh 0)
    (if (Rendering|IsVisible _widget)
      (Development|SetHiddeninGame _widget true false))))

(event Custom|Open%20Door%20%28multicast%29
  (params (Locked :type Integer))
  (bind _sm_door_handle_003 (Variables|Default|GetSM_door_handle_003))
  (bind _returnvalue (Transformation|GetWorldLocation _sm_door_handle_003))
  ;[1 1 1 0.5] Open Door (multicast)
  (switch int Locked
    (:Default
      (Variables|Default|SetLocked false)
      (Default|DetachItem (Variables|Default|GetPlayer) true)
      (Audio|PlaySoundatLocation "/Game/ACaseOfMurder/Audio/Interaction/MSS_DoorUnlock.MSS_DoorUnlock" _returnvalue "0, 0, 0" 1.0 1.0 0.0 0 0 0 0))
    (:0
      (Audio|PlaySoundatLocation "/Game/ACaseOfMurder/Audio/Interaction/MSS_DoorOpen.MSS_DoorOpen" _returnvalue "0, 0, 0" 1.0 1.0 0.0 0 0 0 0)
      (Class|EnhancedInputSubsystemInterface|ClearAllMappings (PlayerController|LocalPlayerSubsystems|GetEnhancedInputLocalPlayerSubsystem (Game|GetPlayerController 0)))
      (bind _returnvalue_2 (Actor|GetActorOfClass "/Script/Engine.PostProcessVolume"))
      (Utilities|Struct|SetmembersinPostProcessSettings (Variables|/Script/Engine.PostProcessVolume|GetSettings _returnvalue_2) (Variables|Default|GetBlackscreen))
      (bind _foundwidgets (Widget|GetAllWidgetsOfClass "/Script/UMG.UserWidget" true))
      (for _array_element _foundwidgets
        (Widget|SetVisibility _array_element "Hidden")
        (bind _returnvalue_3 (Actor|GetActorOfClass "/Game/ACaseOfMurder/Blueprints/BP_DialogueManager.BP_DialogueManager_C"))
        (bind _outactors (Actor|GetAllActorsOfClass "/Script/Engine.AmbientSound"))
        (for _array_element_2 _outactors
          (Audio|Components|Audio|AdjustVolume (Variables|/Script/Engine.AmbientSound|GetAudioComponent _array_element_2) 1.0 0.05 "Linear" :!class /Script/Engine.AudioComponent)
          (Default|StartDialogue _returnvalue_3 "/Game/ACaseOfMurder/Data/DA_Dialogue_EndCorrect.DA_Dialogue_EndCorrect")
          (Utilities|FlowControl|Delay 1e+01)
          (Game|QuitGame 0 "Quit" false))))
    (:1
      (Audio|PlaySoundatLocation "/Game/ACaseOfMurder/Audio/Interaction/MSS_DoorTryOpen.MSS_DoorTryOpen" _returnvalue "0, 0, 0" 1.0 1.0 0.0 0 0 0 0))))

(event EventBeginPlay
  ;[1 1 1 0.5] Begin Play
  (bind _aswbp_nearest_interaction (Utilities|Casting|CastToWBP_NearestInteraction (UserInterface|GetWidget (Variables|Default|GetWidget))))
  (Variables|Default|SetAs%20WBP%20Nearest%20Interaction _aswbp_nearest_interaction)
  (Utilities|FlowControl|DelayUntilNextTick)
  (bind _asbp_interaction_character (Utilities|Casting|CastToBP_InteractionCharacter (Game|Player|GetPlayerPawn 0)))
  (Variables|Default|SetPlayer _asbp_interaction_character))

(event EventFocusInteraction
  (params (Focused :type Boolean))
  (bind _widget (Variables|Default|GetWidget))
  (bind _widget_2 (Variables|Default|GetWidget))
  (bind _staticmesh (Variables|Default|GetStaticMesh))
  ;[1 1 1 0.5] Focus Interaction (interface)
  (if Focused
    ;[0.6445 0.8228 1 0.502] Local Visual
    (Rendering|SetRenderCustomDepth _staticmesh true)
    (Rendering|SetCustomDepthStencilValue _staticmesh 2)
    (if (Rendering|IsVisible _widget_2)
      _
      (else
        (Development|SetHiddeninGame _widget_2 false false)))
    (Default|OnFocused (Variables|Default|GetAs%20WBP%20Nearest%20Interaction) true)
    (else
      (Rendering|SetRenderCustomDepth _staticmesh false)
      (Rendering|SetCustomDepthStencilValue _staticmesh 0)
      (if (Rendering|IsVisible _widget)
        _
        (else
          (Development|SetHiddeninGame _widget true false)))
      (Default|OnFocused (Variables|Default|GetAs%20WBP%20Nearest%20Interaction) false))))

(event EventInteractwithActor
  ;[1 1 1 0.5] Interact With Actor (interface)
  (CallFunction|OpenDoor(multicast) (+ (Math|Conversions|ToInteger(Boolean) (Variables|Default|GetLocked)) (Math|Conversions|ToInteger(Boolean) (== (Variables|/Game/Fab/InteractionSystem/Character/BP_InteractionCharacter.BP_InteractionCharacter_C|GetHeld%20Item (Variables|Default|GetPlayer)) (Variables|Default|GetKey))))))

(fn ConstructionScript
  (Components|Sphere|SetSphereRadius (Variables|Default|GetSphere) (Variables|/Game/ACaseOfMurder/Data/BP_FloatData.BP_FloatData_C|GetValue (Variables|Default|GetMaxDistance)) true))