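; Dialogue manager that plays sequenced voice lines from Diego (the player), the Boss and recordings, starting with the intro on BeginPlay.
; It steps through the current dialogue asset's entries, routing each sound and delay to the matching character or to all speakers at once.
; Audio-finished events from both characters and only the first speaker advance the sequence.
; A gate briefly blocks advancing whenever a new dialogue starts.
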(event Custom|Play%20Speakers
  (params (Audio%20File :type Sound%20Wave%20Object%20Reference) (Delay :type Float%20%28double-precision%29))
  ;[0.15 0.5 0.1 0.5] Play Audio File from all speakers
  (Utilities|FlowControl|Delay Delay)
  (for _array_element (Variables|References|GetSpeakers)
    (Default|PlayAudio _array_element Audio%20File)))

(event Custom|Start%20Dialogue
  (params (Dialogue :type BP%20Dialogue%20Data%20Object%20Reference))
  (Utilities|FlowControl|Sequence
    (:then_0
      (Utilities|FlowControl|Gate true) ; enters at Close
    )
    (:then_1
      (Variables|Default|SetCurrent%20Dialogue Dialogue)
      (bind _output_get (Variables|Default|SetIndex 0))
      (switch Utilities|FlowControl|Switch|SwitchonE_Speaker (.speaker (Utilities|Array|Get(acopy) (Variables|/Game/ACaseOfMurder/Data/BP_DialogueData.BP_DialogueData_C|GetData (Variables|Default|GetCurrent%20Dialogue)) _output_get))
        (:NewEnumerator0
          (Default|PlayDialogue (Variables|References|GetPlayer) (.soundwave (Utilities|Array|Get(acopy) (Variables|/Game/ACaseOfMurder/Data/BP_DialogueData.BP_DialogueData_C|GetData (Variables|Default|GetCurrent%20Dialogue)) _output_get)) (.delay (Utilities|Array|Get(acopy) (Variables|/Game/ACaseOfMurder/Data/BP_DialogueData.BP_DialogueData_C|GetData (Variables|Default|GetCurrent%20Dialogue)) _output_get))))
        (:NewEnumerator1
          (Default|PlayDialogue (Variables|References|GetBoss) (.soundwave (Utilities|Array|Get(acopy) (Variables|/Game/ACaseOfMurder/Data/BP_DialogueData.BP_DialogueData_C|GetData (Variables|Default|GetCurrent%20Dialogue)) _output_get)) (.delay (Utilities|Array|Get(acopy) (Variables|/Game/ACaseOfMurder/Data/BP_DialogueData.BP_DialogueData_C|GetData (Variables|Default|GetCurrent%20Dialogue)) _output_get))))
        (:NewEnumerator2
          (CallFunction|PlaySpeakers (.soundwave (Utilities|Array|Get(acopy) (Variables|/Game/ACaseOfMurder/Data/BP_DialogueData.BP_DialogueData_C|GetData (Variables|Default|GetCurrent%20Dialogue)) _output_get)) (.delay (Utilities|Array|Get(acopy) (Variables|/Game/ACaseOfMurder/Data/BP_DialogueData.BP_DialogueData_C|GetData (Variables|Default|GetCurrent%20Dialogue)) _output_get))))))
    (:then_2
      (Utilities|FlowControl|Delay 1.0)
      (Utilities|FlowControl|Gate true) ; enters at Open
    )))

(event Custom|Next%20Speaker
  (bind _index (Variables|Default|GetIndex))
  (bind _current_dialogue (Variables|Default|GetCurrent%20Dialogue))
  (bind _data (Variables|/Game/ACaseOfMurder/Data/BP_DialogueData.BP_DialogueData_C|GetData _current_dialogue))
  (Utilities|FlowControl|Gate true
    (:Exit
      (Math|Integer|IncrementInt _index
        (:%20%20
          (if (< _index (Utilities|Array|Length _data))
            (switch Utilities|FlowControl|Switch|SwitchonE_Speaker (.speaker (Utilities|Array|Get(acopy) _data (stale Custom|Start%20Dialogue _output_get)))
              (:NewEnumerator0
                (Default|PlayDialogue (Variables|References|GetPlayer) (.soundwave (Utilities|Array|Get(acopy) _data (stale Custom|Start%20Dialogue _output_get))) (.delay (Utilities|Array|Get(acopy) _data (stale Custom|Start%20Dialogue _output_get)))))
              (:NewEnumerator1
                (Default|PlayDialogue (Variables|References|GetBoss) (.soundwave (Utilities|Array|Get(acopy) _data (stale Custom|Start%20Dialogue _output_get))) (.delay (Utilities|Array|Get(acopy) _data (stale Custom|Start%20Dialogue _output_get)))))
              (:NewEnumerator2
                (CallFunction|PlaySpeakers (.soundwave (Utilities|Array|Get(acopy) _data (stale Custom|Start%20Dialogue _output_get))) (.delay (Utilities|Array|Get(acopy) _data (stale Custom|Start%20Dialogue _output_get))))))))))))

(event EventBeginPlay
  (Utilities|FlowControl|DelayUntilNextFrame)
  (Utilities|FlowControl|Sequence
    (:then_0
      (bind _outactors (Actor|GetAllActorsOfClass "/Game/ACaseOfMurder/Blueprints/BP_Speaker.BP_Speaker_C"))
      (bind _output_get (Variables|References|SetSpeakers _outactors))
      (bind _returnvalue (Actor|GetActorOfClass "/Game/ACaseOfMurder/Blueprints/BP_Boss.BP_Boss_C"))
      (bind _output_get_2 (Variables|References|SetBoss _returnvalue))
      (bind _returnvalue_2 (Actor|GetActorOfClass "/Game/Fab/InteractionSystem/Character/BP_InteractionCharacter.BP_InteractionCharacter_C"))
      (bind _output_get_3 (Variables|References|SetPlayer _returnvalue_2)))
    (:then_1
      (EventDispatchers|BindEventtoOnAudioFinished (Variables|/Game/ACaseOfMurder/Blueprints/BP_Speaker.BP_Speaker_C|GetMSS_SpeakerAudio (Utilities|Array|Get(acopy) _output_get)) (delegate Custom|Next%20Speaker))
      (EventDispatchers|BindEventtoOnAudioFinished (Variables|/Game/ACaseOfMurder/Blueprints/BP_Boss.BP_Boss_C|GetMSS_DialoguePlayer _output_get_2) (delegate Custom|Next%20Speaker))
      (EventDispatchers|BindEventtoOnAudioFinished (Variables|/Game/Fab/InteractionSystem/Character/BP_InteractionCharacter.BP_InteractionCharacter_C|GetMSS_DialoguePlayer _output_get_3) (delegate Custom|Next%20Speaker))
      (Utilities|FlowControl|Delay 0.2)
      (CallFunction|StartDialogue "/Game/ACaseOfMurder/Data/DA_Dialogue_Intro.DA_Dialogue_Intro"))))

(fn ConstructionScript)