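; BP_CeilingFan is a ceiling fan prop with a spotlight and audio for the fan and lamp hum.
; The construction script applies the configured light intensity and sets the Gain parameter on both sound components from their volume variables.
; Tick yaws the Fan component in local space, scaled by delta time, so SpinRate reads as revolutions per second.
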(event EventBeginPlay)

(event Collision|EventActorBeginOverlap
  (params (OtherActor :type Actor%20Object%20Reference)))

(event EventTick
  (params (DeltaSeconds :type Float%20%28single-precision%29))
  (Transformation|AddLocalRotation (Variables|Default|GetFan) (Math|Rotator|MakeRotator 0.0 0.0 (* DeltaSeconds (Variables|Default|GetSpin%20rate) 3.6e+02)) false false))

(fn ConstructionScript
  (Rendering|Components|Light|SetIntensity (Variables|Default|GetSpotLight) (Variables|Default|GetLight%20Intensity))
  (Audio|Parameter|SetFloatParameter (Variables|Default|GetMSS_LampHum) "Gain" (Variables|Default|GetHum%20Volume) :!class /Script/Engine.AudioComponent)
  (Audio|Parameter|SetFloatParameter (Variables|Default|GetMSS_CeilingFan) "Gain" (Variables|Default|GetFan%20Volume) :!class /Script/Engine.AudioComponent))