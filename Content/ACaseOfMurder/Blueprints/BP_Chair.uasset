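; Interactable chair that the player can sit on and stand up from.
; A sphere overlap and interface focus events drive a prompt widget and custom-depth outline.
; Interacting toggles the seated state, swaps controller input and fires a multicast that plays a sound and acts on player 0.
; Chained timelines move and attach the pawn to the seat, then shift the chair while turning the view toward a look target, reversing to stand.
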(event OnComponentBeginOverlap(Sphere)
  (params (OverlappedComponent :type Primitive%20Component%20Object%20Reference) (OtherActor :type Actor%20Object%20Reference) (OtherComp :type Primitive%20Component%20Object%20Reference) (OtherBodyIndex :type Integer) (bFromSweep :type Boolean) (SweepResult :type Hit%20Result%20Structure%20%28by%20ref%29))
  ;[0.6445 0.8228 1 0.502] Local Overlap Event
  (if (== (Game|GetPlayerCharacter 0) OtherActor)
    (Utilities|Casting|CastToBP_InteractionCharacter OtherActor)
    (Development|SetHiddeninGame (Variables|Default|GetWidget) false false)))

(event OnComponentEndOverlap(Sphere)
  (params (OverlappedComponent :type Primitive%20Component%20Object%20Reference) (OtherActor :type Actor%20Object%20Reference) (OtherComp :type Primitive%20Component%20Object%20Reference) (OtherBodyIndex :type Integer))
  (bind _chair (Variables|Default|GetChair))
  (bind _widget (Variables|Default|GetWidget))
  ;[0.6445 0.8228 1 0.502] Local Overlap Event
  (if (== OtherActor (Game|GetPlayerCharacter 0))
    (Utilities|Casting|CastToBP_InteractionCharacter OtherActor)
    (Rendering|SetRenderCustomDepth _chair false)
    (Rendering|SetCustomDepthStencilValue _chair 0)
    (if (Rendering|IsVisible _widget)
      (Development|SetHiddeninGame _widget true false))))

(event Custom|Sit%20%28multicast%29
  (params (Sat :type Boolean))
  (bind _returnvalue (Game|Player|GetPlayerPawn 0))
  ;[1 1 1 0.5] Open Door (multicast)
  (Audio|PlaySoundatLocation "/Game/ACaseOfMurder/Audio/Interaction/MSS_ChairSit.MSS_ChairSit" (Transformation|GetWorldLocation (Variables|Default|GetChair)) "0, 0, 0" 1.0 1.0 0.0 0 0 0 0)
  (if Sat
    (Collision|SetActorEnableCollision _returnvalue false)
    (Variables|Default|SetStanding%20Transform (Transformation|GetActorTransform _returnvalue))
    (Audio|Components|Audio|Play (Variables|Default|GetSit%20Timeline))
    (else
      (Utilities|String|Reverse (Variables|Default|GetChair%20Timeline)))))

(event EventBeginPlay
  ;[1 1 1 0.5] Begin Play
  (bind _aswbp_nearest_interaction (Utilities|Casting|CastToWBP_NearestInteraction (UserInterface|GetWidget (Variables|Default|GetWidget))))
  (Variables|Default|SetAs%20WBP%20Nearest%20Interaction _aswbp_nearest_interaction))

(event EventFocusInteraction
  (params (Focused :type Boolean))
  (bind _chair (Variables|Default|GetChair))
  (bind _widget (Variables|Default|GetWidget))
  (bind _widget_2 (Variables|Default|GetWidget))
  ;[1 1 1 0.5] Focus Interaction (interface)
  (if Focused
    ;[0.6445 0.8228 1 0.502] Local Visual
    (Rendering|SetRenderCustomDepth _chair true)
    (Rendering|SetCustomDepthStencilValue _chair 2)
    (if (Rendering|IsVisible _widget_2)
      _
      (else
        (Development|SetHiddeninGame _widget_2 false false)))
    (Default|OnFocused (Variables|Default|GetAs%20WBP%20Nearest%20Interaction) true)
    (else
      (Rendering|SetRenderCustomDepth _chair false)
      (Rendering|SetCustomDepthStencilValue _chair 0)
      (if (Rendering|IsVisible _widget)
        _
        (else
          (Development|SetHiddeninGame _widget true false)))
      (Default|OnFocused (Variables|Default|GetAs%20WBP%20Nearest%20Interaction) false))))

(event EventInteractwithActor
  ;[1 1 1 0.5] Interact With Actor (interface)
  (bind _asbp_interaction_pc (Utilities|Casting|CastToBP_Interaction_PC (Game|GetPlayerController 0)))
  (if (Variables|Default|GetSat)
    (Variables|Default|SetSat false)
    (else
      (bind _output_get (Variables|Default|SetSat true))))
  (Default|SwapInput _asbp_interaction_pc _output_get)
  (CallFunction|Sit(multicast) _output_get)
  ;[0.15 0.15 0.15 0.5] Get player camera
  (Utilities|FlowControl|Sequence
    (:then_0
      (Utilities|FlowControl|Gate false :!label _label
        (:Exit
          (bind _asbp_interaction_character (Utilities|Casting|CastToBP_InteractionCharacter (Game|Player|GetPlayerPawn 0)))
          (Variables|Default|SetCamera (Variables|/Game/Fab/InteractionSystem/Character/BP_InteractionCharacter.BP_InteractionCharacter_C|GetCamera _asbp_interaction_character))
          (bind _asbp_interaction_pc_2 (Utilities|Casting|CastToBP_Interaction_PC (Game|GetPlayerController 0)))
          (Variables|/Game/Fab/InteractionSystem/Core/BP_Interaction_PC.BP_Interaction_PC_C|SetLook%20Target _asbp_interaction_pc_2 (Transformation|GetWorldLocation (Variables|Default|GetLook%20Target))))))
    (:then_1
      (goto _label Close))))

(fn ConstructionScript
  (Components|Sphere|SetSphereRadius (Variables|Default|GetSphere) (Variables|/Game/ACaseOfMurder/Data/BP_FloatData.BP_FloatData_C|GetValue (Variables|Default|GetMaxDistance)) true))