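; An interactable computer prop whose monitor the player can switch on and off.
; The interact interface event flips Lit and calls a multicast event that swaps the monitor material and plays or reverses a timeline driving the monitor light intensity.
; A sphere overlap shows the prompt widget to the local player character, while the focus interface event highlights the tower through custom depth stencil and notifies the widget.
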(event OnComponentBeginOverlap(Sphere)
  (params (OverlappedComponent :type Primitive%20Component%20Object%20Reference) (OtherActor :type Actor%20Object%20Reference) (OtherComp :type Primitive%20Component%20Object%20Reference) (OtherBodyIndex :type Integer) (bFromSweep :type Boolean) (SweepResult :type Hit%20Result%20Structure%20%28by%20ref%29))
  ;[0.6445 0.8228 1 0.502] Local Overlap Event
  (if (== (Game|GetPlayerCharacter 0) OtherActor)
    (Utilities|Casting|CastToBP_InteractionCharacter OtherActor)
    (Development|SetHiddeninGame (Variables|Default|GetWidget) false false)))

(event OnComponentEndOverlap(Sphere)
  (params (OverlappedComponent :type Primitive%20Component%20Object%20Reference) (OtherActor :type Actor%20Object%20Reference) (OtherComp :type Primitive%20Component%20Object%20Reference) (OtherBodyIndex :type Integer))
  (bind _sm_computertower_b01_n1 (Variables|Default|GetSM_ComputerTower_B01_N1))
  (bind _widget (Variables|Default|GetWidget))
  ;[0.6445 0.8228 1 0.502] Local Overlap Event
  (if (== OtherActor (Game|GetPlayerCharacter 0))
    (Utilities|Casting|CastToBP_InteractionCharacter OtherActor)
    (Rendering|SetRenderCustomDepth _sm_computertower_b01_n1 false)
    (Rendering|SetCustomDepthStencilValue _sm_computertower_b01_n1 0)
    (if (Rendering|IsVisible _widget)
      (Development|SetHiddeninGame _widget true false))))

(event Custom|Switch%20Light%20%28multicast%29
  (params (Lit :type Boolean))
  (bind _sm_computermonitor_a01_n1 (Variables|Default|GetSM_ComputerMonitor_A01_N1))
  (bind _timeline (Variables|Default|GetTimeline))
  ;[1 1 1 0.5] Open Door (multicast)
  (if Lit
    (Utilities|String|Reverse _timeline)
    (Rendering|Material|SetMaterial _sm_computermonitor_a01_n1 0 (Variables|Default|GetMonitor%20Lit))
    (else
      (Audio|Components|Audio|Play _timeline)
      (Rendering|Material|SetMaterial _sm_computermonitor_a01_n1 0 (Variables|Default|GetMonitor%20Unlit)))))

(event EventBeginPlay
  ;[1 1 1 0.5] Begin Play
  (bind _aswbp_nearest_interaction (Utilities|Casting|CastToWBP_NearestInteraction (UserInterface|GetWidget (Variables|Default|GetWidget))))
  (Variables|Default|SetAs%20WBP%20Nearest%20Interaction _aswbp_nearest_interaction))

(event EventFocusInteraction
  (params (Focused :type Boolean))
  (bind _widget (Variables|Default|GetWidget))
  (bind _widget_2 (Variables|Default|GetWidget))
  (bind _sm_computertower_b01_n1 (Variables|Default|GetSM_ComputerTower_B01_N1))
  ;[1 1 1 0.5] Focus Interaction (interface)
  (if Focused
    ;[0.6445 0.8228 1 0.502] Local Visual
    (Rendering|SetRenderCustomDepth _sm_computertower_b01_n1 true)
    (Rendering|SetCustomDepthStencilValue _sm_computertower_b01_n1 2)
    (if (Rendering|IsVisible _widget_2)
      _
      (else
        (Development|SetHiddeninGame _widget_2 false false)))
    (Default|OnFocused (Variables|Default|GetAs%20WBP%20Nearest%20Interaction) true)
    (else
      (Rendering|SetRenderCustomDepth _sm_computertower_b01_n1 false)
      (Rendering|SetCustomDepthStencilValue _sm_computertower_b01_n1 0)
      (if (Rendering|IsVisible _widget)
        _
        (else
          (Development|SetHiddeninGame _widget true false)))
      (Default|OnFocused (Variables|Default|GetAs%20WBP%20Nearest%20Interaction) false))))

(event EventInteractwithActor
  ;[1 1 1 0.5] Interact With Actor (interface)
  (if (Variables|Default|GetLit)
    (Variables|Default|SetLit false)
    (else
      (Variables|Default|SetLit true)))
  (CallFunction|SwitchLight(multicast) (Variables|Default|GetLit)))

(fn ConstructionScript)